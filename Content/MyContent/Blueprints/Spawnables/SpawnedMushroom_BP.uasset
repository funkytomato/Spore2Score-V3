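; A self-propagating mushroom that seeds interactable adult mushrooms and copies of itself at random points within a proximity radius.
; A one-shot timer spawns the adult if the cap allows, while a looping timer endlessly spawns babies that inherit its mushroom classes and repeat the cycle.
; The first four babies get an adult cap of zero; every later one gets one, despite comments saying every fifth.
; An unconnected overlap check would flag nearby interactables as mushroomed.
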(event `self.ReceiveBeginPlay`
  ;[1 1 1] Initialise Timer for Spawning adult interactable mushroom
  (bind _returnvalue (`KismetSystemLibrary.K2_SetTimerDelegate` (delegate `SpawnMushroomInteractable`) 5.0 false 0.0 3.0))
  (set `self.MushroomSpawnTimerRef` _returnvalue)
  ;[1 1 1] Initialise Timer for spawning baby mushrooms
  (bind _returnvalue_2 (`KismetSystemLibrary.K2_SetTimerDelegate` (delegate `SpawnBabyMushroom`) 5.0 true 5.0 5.0))
  (set `self.BabyMushroomSpawnerTimerRef` _returnvalue_2))

(event `SpawnMushroomInteractable`
  (bind (_returnvalue_x _returnvalue_y _returnvalue_z) (`KismetMathLibrary.BreakVector` (`self.K2_GetActorLocation`)))
  ;[1 1 1] Initialise Timer for Spawning adult interactable mushroom
  ;[1 1 1] Spawn Adult Interactable Mushroom
  (if (< (`self.SpawnAdultMushroomCount`) (`self.MaxSpawnAdultMushroomTotal`))
    (`|SpawnActorFromClass` (`self.SpawnMushroomBP`) (`KismetMathLibrary.MakeTransform` (`KismetMathLibrary.MakeVector` (`KismetMathLibrary.RandomFloatInRange` (- _returnvalue_x (`self.ProximityRadius`)) (+ _returnvalue_x (`self.ProximityRadius`))) (`KismetMathLibrary.RandomFloatInRange` (- _returnvalue_y (`self.ProximityRadius`)) (+ _returnvalue_y (`self.ProximityRadius`))) _returnvalue_z) (`SceneComponent.K2_GetComponentRotation` (`self.DefaultSceneRoot`))) "AdjustIfPossibleButAlwaysSpawn" "OverrideRootScale" null null)
    ;[1 1 1] Increment Mushroom Spawn Count
    (set `self.SpawnAdultMushroomCount` (+ (`self.SpawnAdultMushroomCount`) 1))
    (else
      (`KismetSystemLibrary.K2_ClearAndInvalidateTimerHandle` (`self.MushroomSpawnTimerRef`)))))

(event `SpawnBabyMushroom`
  (bind (_returnvalue_x _returnvalue_y _returnvalue_z) (`KismetMathLibrary.BreakVector` (`self.K2_GetActorLocation`)))
  ;[1 1 1] Spawn Baby Mushroom
  (set `self.SpawnBabyMushroomCount` (+ (`self.SpawnBabyMushroomCount`) 1))
  ;;[1 1 1] Spawn Baby mushroom, set the class and set adult mushroom spawn to 0 (Do not want lots of interactable mushrooms!!!!)
  (bind _returnvalue (`|SpawnActorFromClass` "SpawnedMushroom_BP_C" (`KismetMathLibrary.MakeTransform` (`KismetMathLibrary.MakeVector` (`KismetMathLibrary.RandomFloatInRange` (- _returnvalue_x (`self.ProximityRadius`)) (+ _returnvalue_x (`self.ProximityRadius`))) (`KismetMathLibrary.RandomFloatInRange` (- _returnvalue_y (`self.ProximityRadius`)) (+ _returnvalue_y (`self.ProximityRadius`))) _returnvalue_z) (`SceneComponent.K2_GetComponentRotation` (`self.DefaultSceneRoot`))) "AdjustIfPossibleButDontSpawnIfColliding" "OverrideRootScale" null null))
  (set `/Game/MyContent/Blueprints/Spawnables/SpawnedMushroom_BP.MushroomClass` (`self.MushroomClass`) _returnvalue)
  (set `/Game/MyContent/Blueprints/Spawnables/SpawnedMushroom_BP.SpawnMushroomBP` (`self.SpawnMushroomBP`) _returnvalue)
  (if (== (/ (`self.SpawnBabyMushroomCount`) 5) 0)
    ;;[1 1 1] Do not spawn Adult Mushroom
    (set `/Game/MyContent/Blueprints/Spawnables/SpawnedMushroom_BP.MaxSpawnAdultMushroomTotal` 0 _returnvalue)
    (else
      ;;[1 1 1] Spawn Adult Mushroom every 5 baby mushrooms spawned
      (set `/Game/MyContent/Blueprints/Spawnables/SpawnedMushroom_BP.MaxSpawnAdultMushroomTotal` 1 _returnvalue))))

(fn `UserConstructionScript`)