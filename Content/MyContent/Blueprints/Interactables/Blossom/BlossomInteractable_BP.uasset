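; Interactable blossom plant whose look follows its health across Blossom, OK, Dying and Dead states.
; A bound HealthBoost event adds to the clamped health, maps it to a status by thresholds, then updates visuals.
; DoOnce gates that reset neighboring states limit repeat swaps of leaf materials, or of mesh and branch material when dead.
; Health between zero and the Dying threshold only prints an error, leaving status unchanged.
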(event `UpdateVisuals`
  (bind _interactablesm (`self.InteractableSM`))
  (switch `/Game/MyContent/Blueprints/Interactables/Blossom/BlossomHealth` (`self.HealthStatus`)
    (:`NewEnumerator0`
      (`/Engine/EditorBlueprintResources/StandardMacros.DoOnce` false :!label _label
        (:`Completed`
          (`PrimitiveComponent.SetMaterialByName` (`self.InteractableSM`) "Leaves" (`self.BlossomMaterialName`))
          (`|ExecutionSequence`
            (:`then_0`
              (goto _label_2 :!via `Reset`))
            (:`then_1`
              (goto _label_3 :!via `Reset`))))))
    (:`NewEnumerator1`
      (`/Engine/EditorBlueprintResources/StandardMacros.DoOnce` false :!label _label_2
        (:`Completed`
          (`PrimitiveComponent.SetMaterialByName` (`self.InteractableSM`) "Leaves" (`self.OKMaterialName`))
          (`|ExecutionSequence`
            (:`then_0`
              (goto _label :!via `Reset`))
            (:`then_1`
              (goto _label_3 :!via `Reset`))))))
    (:`NewEnumerator2`
      (`/Engine/EditorBlueprintResources/StandardMacros.DoOnce` false :!label _label_3
        (:`Completed`
          (`PrimitiveComponent.SetMaterialByName` (`self.InteractableSM`) "Leaves" (`self.DyingMaterialName`))
          (`|ExecutionSequence`
            (:`then_0`
              (goto _label_2 :!via `Reset`))
            (:`then_1`
              (goto _label_4 :!via `Reset`))))))
    (:`NewEnumerator3`
      (`/Engine/EditorBlueprintResources/StandardMacros.DoOnce` false :!label _label_4
        (:`Completed`
          (`StaticMeshComponent.SetStaticMesh` _interactablesm (`self.DeadMesh`))
          (`PrimitiveComponent.SetMaterialByName` _interactablesm "Branches" (`self.DeadMaterialName`))
          (`|ExecutionSequence`
            (:`then_0`
              (goto _label_3 :!via `Reset`))))))))

(event `self.ReceiveBeginPlay`
  (`parent.ReceiveBeginPlay`)
  (add `self.HealthBoost` (delegate `HealthBoost_Event`)))

(event `HealthBoost_Event` :!signature `self.HealthBoost`
  (params (BoostAmount :type "Float (double-precision)"))
  (`self.UpdateHealthStatus` (`KismetMathLibrary.FClamp` (+ (`self.Health`) BoostAmount) 0.0 100.0))
  (`self.UpdateVisuals`))

(fn `UpdateHealthStatus`
  (params (Health :type "Float (double-precision)"))
  (bind _output_get (set `self.Health` Health))
  (if (>= _output_get 100.0)
    (set `self.HealthStatus` "NewEnumerator0")
    (elif (>= _output_get 75.0)
      (set `self.HealthStatus` "NewEnumerator1")
      (elif (>= _output_get 50.0)
        (set `self.HealthStatus` "NewEnumerator2")
        (elif (<= _output_get 0.0)
          (set `self.HealthStatus` "NewEnumerator3")
          (else
            (`KismetSystemLibrary.PrintString` "HealthBoost invalid healthboost")))))))

(fn `UserConstructionScript`
  (`parent.UserConstructionScript`))