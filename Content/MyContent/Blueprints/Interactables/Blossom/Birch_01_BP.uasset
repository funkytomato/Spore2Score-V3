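; Birch tree interactable Blueprint in the Blossom folder that steadily loses health over time, apparently as a test of health decay.
; A looping timer started on BeginPlay periodically subtracts a fixed amount from Health, passes a clamped copy to UpdateHealthStatus, then calls UpdateVisuals.
; The Health variable itself is never clamped here, and the construction script only calls the parent.
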(event `self.ReceiveBeginPlay`
  (`parent.ReceiveBeginPlay`)
  (`KismetSystemLibrary.K2_SetTimerDelegate` (delegate `DecreaseHealthEventTest`) 2.0 true))

(event `DecreaseHealthEventTest`
  (bind _output_get (set `self.Health` (- (`self.Health`) 5.0)))
  (`self.UpdateHealthStatus` (`KismetMathLibrary.FClamp` _output_get 0.0 100.0))
  (`self.UpdateVisuals`))

(fn `UserConstructionScript`
  (`parent.UserConstructionScript`))