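; Interactable bush that shows its health status by changing colour and sinks away when it dies.
; It binds to the parent's health boost dispatcher and switches on HealthStatus to play a matching timeline.
; Blossom, OK and Dying timelines lerp the TreeColour parameter of a dynamic material created in the construction script.
; Dead runs once, lowering the actor into the ground, then setting a short lifespan to remove it.
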(event `self.ReceiveBeginPlay`
  (`parent.ReceiveBeginPlay`)
  ;[1 1 1] Assign Health Boost Despatch Message and Update Visuals
  (add `self.HealthBoost` (delegate `UpdateVisuals`)))

(event `UpdateVisuals` :!signature `self.HealthBoost`
  (params (BoostAmount :type "Float (double-precision)"))
  ;[1 1 1] Assign Health Boost Despatch Message and Update Visuals
  (switch `/Game/MyContent/Blueprints/Interactables/Blossom/BlossomHealth` (`self.HealthStatus`)
    (:`NewEnumerator0`
      (`self.UpdateBlossomVisual`))
    (:`NewEnumerator1`
      (`self.UpdateOKVisual`))
    (:`NewEnumerator2`
      (`self.UpdateDyingVisual`))
    (:`NewEnumerator3`
      (`self.UpdateDeadVisual`))))

(event `UpdateBlossomVisual`
  ;[1 1 1] Change Visuals to Blossom
  (bind (_direction _alpha) (`Timeline|BlossomTimeline` :!via `PlayFromStart`)
    (:`Update`
      (bind _returnvalue (`MaterialInstanceDynamic.K2_GetVectorParameterValue` (`self.DynamicMaterial`) "TreeColour"))
      (`MaterialInstanceDynamic.SetVectorParameterValue` (`self.DynamicMaterial`) "TreeColour" (`KismetMathLibrary.LinearColorLerp` _returnvalue (struct :`R` 0.051351 :`G` 0.896255 :`A` 1.0) _alpha)))))

(event `UpdateOKVisual`
  ;[1 1 1] Change Visuals to OK
  (bind (_direction _alpha) (`Timeline|OKTimeline` :!via `PlayFromStart`)
    (:`Update`
      (bind _returnvalue (`MaterialInstanceDynamic.K2_GetVectorParameterValue` (`self.DynamicMaterial`) "TreeColour"))
      (`MaterialInstanceDynamic.SetVectorParameterValue` (`self.DynamicMaterial`) "TreeColour" (`KismetMathLibrary.LinearColorLerp` _returnvalue (struct :`R` 0.014388 :`G` 0.372875 :`A` 1.0) _alpha)))))

(event `UpdateDyingVisual`
  ;[1 1 1] Change Visuals to Dying
  (bind (_direction _alpha) (`Timeline|DyingTimeline` :!via `PlayFromStart`)
    (:`Update`
      (bind _returnvalue (`MaterialInstanceDynamic.K2_GetVectorParameterValue` (`self.DynamicMaterial`) "TreeColour"))
      (`MaterialInstanceDynamic.SetVectorParameterValue` (`self.DynamicMaterial`) "TreeColour" (`KismetMathLibrary.LinearColorLerp` _returnvalue (struct :`R` 0.105046 :`G` 0.070604 :`B` 0.013181 :`A` 1.0) _alpha)))))

(event `UpdateDeadVisual`
  (bind (_returnvalue_x _returnvalue_y _returnvalue_z) (`KismetMathLibrary.BreakVector` (`self.K2_GetActorLocation`)))
  ;[1 1 1] Change Visuals to Dead
  (`/Engine/EditorBlueprintResources/StandardMacros.DoOnce` false
    (:`Completed`
      (bind (_direction _alpha) (`Timeline|DisappearIntoGround` :!via `PlayFromStart`)
        (:`Update`
          (`self.K2_SetActorLocation` (`KismetMathLibrary.VLerp` (`KismetMathLibrary.MakeVector` _returnvalue_x _returnvalue_y _returnvalue_z) (`KismetMathLibrary.MakeVector` _returnvalue_x _returnvalue_y -250.0) _alpha)))
        (:`Finished`
          (`self.SetLifeSpan` 1.0))))))

(fn `UserConstructionScript`
  (`parent.UserConstructionScript`)
  (bind _returnvalue (`PrimitiveComponent.CreateDynamicMaterialInstance` (`self.InteractableSM`) 0 null "None"))
  (bind _output_get (set `self.DynamicMaterial` _returnvalue))
  (`PrimitiveComponent.SetMaterial` (`self.InteractableSM`) 0 _output_get))