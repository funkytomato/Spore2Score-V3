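; Base interactable Blueprint with a radius of influence and a status widget, for mushroom effects on surrounding vegetation.
; After a short BeginPlay delay, it caches overlapping interactables, links the widget to itself and sets a zero-time timer on the boost event.
; That event is written to boost Blossom health or decrease Debris health for matching influence types, though its loop shows no input array.
; Player overlap toggles the widget, rotated toward the camera upon entry.
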(event `self.ReceiveBeginPlay`
  ;[1 1 1] Get List Of Nearby Interactables
  (`KismetSystemLibrary.Delay` 0.2)
  (set `self.InteractablesNearby` (`PrimitiveComponent.GetOverlappingActors` (`self.RadiusOfInfluence`) "MasterInteractable_BP_C"))
  ;[1 1 1] Timer for HealthBoost or HealthDeplete
  (`KismetSystemLibrary.K2_SetTimerDelegate` (delegate `HealthBoostToSurroundingVegetation`))
  ;[1 1 1] Assign Status Widget
  (bind _asinteractable_status_wbp (cast `/Game/MyContent/Widgets/InteractableStatus_WBP` (`WidgetComponent.GetUserWidgetObject` (`self.StatusWidget`))))
  (set `/Game/MyContent/Widgets/InteractableStatus_WBP.OwningActor` self _asinteractable_status_wbp))

(event `HealthBoostToSurroundingVegetation`
  (bind _nutrientboost (`self.NutrientBoost`))
  ;[1 1 1] Timer for HealthBoost or HealthDeplete
  (for _array_element _
    ;[1 1 1] Is MasterInteractable and is correct mushroom type
    (bind _asmaster_interactable_bp (cast `/Game/MyContent/Blueprints/Interactables/MasterInteractable_BP` _array_element))
    (if (`|EnumEquality` (`/Game/MyContent/Blueprints/Interactables/MasterInteractable_BP.MushroomInfluenceType` _asmaster_interactable_bp) (`self.MushroomInfluenceType`))
      (bind _interactabletype (`/Game/MyContent/Blueprints/Interactables/MasterInteractable_BP.InteractableType` _asmaster_interactable_bp))
      ;[1 1 1] Apply effects of mushroom on actor
      (if (`|EnumEquality` _interactabletype "NewEnumerator0")
        (bind _asblossom_interactable_bp (cast `/Game/MyContent/Blueprints/Interactables/Blossom/BlossomInteractable_BP` _asmaster_interactable_bp))
        (`/Game/MyContent/Blueprints/Interactables/Blossom/BlossomInteractable_BP.HealthBoost` _asblossom_interactable_bp _nutrientboost)
        (elif (`|EnumEquality` _interactabletype "NewEnumerator1")
          (bind _asdebris_interactable_bp (cast `/Game/MyContent/Blueprints/Interactables/Debris/DebrisInteractable_BP` _asmaster_interactable_bp))
          (`/Game/MyContent/Blueprints/Interactables/Debris/DebrisInteractable_BP.DecreaseHealth` _asdebris_interactable_bp _nutrientboost)
          (else
            (`KismetSystemLibrary.PrintString` "MasterInteractable - HealthBoostToSurroundingVegetation- Do nothing")))))))

(event `self.RadiusOfInfluence.OnComponentBeginOverlap`
  (params (OverlappedComponent :type "PrimitiveComponent Object Reference") (OtherActor :type "Actor Object Reference") (OtherComp :type "PrimitiveComponent Object Reference") (OtherBodyIndex :type Integer) (bFromSweep :type Boolean) (SweepResult :type "HitResult Structure (by ref)"))
  ;[1 1 1] Show Status Widget on Overlap
  (cast `/Game/TopDownBP/Blueprints/TopDownCharacter` OtherActor)
  (`self.RotateWidgetToFacePlayer`)
  (`SceneComponent.SetVisibility` (`self.StatusWidget`) true false))

(event `self.RadiusOfInfluence.OnComponentEndOverlap`
  (params (OverlappedComponent :type "PrimitiveComponent Object Reference") (OtherActor :type "Actor Object Reference") (OtherComp :type "PrimitiveComponent Object Reference") (OtherBodyIndex :type Integer))
  ;[1 1 1] Show Status Widget on Overlap
  (cast `/Game/TopDownBP/Blueprints/TopDownCharacter` OtherActor)
  (`SceneComponent.SetVisibility` (`self.StatusWidget`) false false))

(fn `RotateWidgetToFacePlayer`
  (bind _astop_down_character (cast `/Game/TopDownBP/Blueprints/TopDownCharacter` (`GameplayStatics.GetPlayerCharacter` 0)))
  (`SceneComponent.K2_SetWorldRotation` (`self.StatusWidget`) (`KismetMathLibrary.FindLookAtRotation` (`SceneComponent.K2_GetComponentLocation` (`self.DefaultSceneRoot`)) (`SceneComponent.K2_GetComponentLocation` (`/Game/TopDownBP/Blueprints/TopDownCharacter.Camera1` _astop_down_character))) false false))

(fn `UserConstructionScript`)