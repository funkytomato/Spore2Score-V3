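; Debris interactable that loses health when its decrease-health event fires and removes itself once depleted.
; On BeginPlay it binds a handler to the DecreaseHealth event, which subtracts the depletion amount and clamps Health to a fixed range.
; At zero health it sets a short life span, so the actor is destroyed after a brief delay.
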(event `self.ReceiveBeginPlay`
  (add `self.DecreaseHealth` (delegate `DecreaseHealth_Event`)))

(event `DecreaseHealth_Event` :!signature `self.DecreaseHealth`
  (params (depleteAmount :type "Float (double-precision)"))
  (bind _output_get (set `self.Health` (`KismetMathLibrary.FClamp` (- (`self.Health`) depleteAmount) 0.0 100.0)))
  (if (<= _output_get 0.0)
    (`self.SetLifeSpan` 3.0)))

(fn `UserConstructionScript`
  (`parent.UserConstructionScript`))