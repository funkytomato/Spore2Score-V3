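; Master Blueprint for a droppable spore that seeds mushroom growth when it touches an interactable.
; On collision overlap with a MasterInteractable_BP implementing InteractableInterface, it spawns an intermediary SpawnedMushroom_BP at the interactable's height, randomly offset in X and Y within Range.
; It passes its spore type and mushroom Blueprint to the spawned mushroom, then sets its own short lifespan to remove itself.
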(event `self.Collision.OnComponentBeginOverlap`
  (params (OverlappedComponent :type "PrimitiveComponent Object Reference") (OtherActor :type "Actor Object Reference") (OtherComp :type "PrimitiveComponent Object Reference") (OtherBodyIndex :type Integer) (bFromSweep :type Boolean) (SweepResult :type "HitResult Structure (by ref)"))
  ;[1 1 1] OnOverlap with Interactable Spawn Intermeditary Mushroom
  ;;[1 1 1] Is Interactable
  (bind _asmaster_interactable_bp (cast `/Game/MyContent/Blueprints/Interactables/MasterInteractable_BP` OtherActor))
  (if (`KismetSystemLibrary.DoesImplementInterface` _asmaster_interactable_bp "/Game/MyContent/Blueprints/Interactables/InteractableInterface.InteractableInterface_C")
    (bind (_returnvalue_x _returnvalue_y _returnvalue_z) (`KismetMathLibrary.BreakVector` (`SceneComponent.K2_GetComponentLocation` (`/Game/MyContent/Blueprints/Interactables/MasterInteractable_BP.DefaultSceneRoot` _asmaster_interactable_bp))))
    ;;[1 1 1] Spawn Intermediary Mushroom and set Mushroom Growth properties
    (bind _returnvalue (`|SpawnActorFromClass` "/Game/MyContent/Blueprints/Spawnables/SpawnedMushroom_BP.SpawnedMushroom_BP_C" (`KismetMathLibrary.MakeTransform` (`KismetMathLibrary.MakeVector` (`KismetMathLibrary.RandomFloatInRange` (- _returnvalue_x (`self.Range`)) (+ _returnvalue_x (`self.Range`))) (`KismetMathLibrary.RandomFloatInRange` (- _returnvalue_y (`self.Range`)) (+ _returnvalue_y (`self.Range`))) _returnvalue_z)) "Undefined" "OverrideRootScale" null null))
    (bind _asspawned_mushroom_bp (cast `/Game/MyContent/Blueprints/Spawnables/SpawnedMushroom_BP` _returnvalue))
    (set `/Game/MyContent/Blueprints/Spawnables/SpawnedMushroom_BP.MushroomClass` (`self.SporeType`) _asspawned_mushroom_bp)
    (set `/Game/MyContent/Blueprints/Spawnables/SpawnedMushroom_BP.SpawnMushroomBP` (`self.MushroomSpawnBP`) _asspawned_mushroom_bp)
    (`self.SetLifeSpan` 2.0)))

(fn `UserConstructionScript`
  (`parent.UserConstructionScript`))